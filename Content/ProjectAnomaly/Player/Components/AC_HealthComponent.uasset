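; Player health component that tracks current health and signals damage and death through event dispatchers.
; Health starts at the maximum on BeginPlay.
; Unless invincible, each TakeDamage call subtracts a hardcoded amount, clamps the result, broadcasts OnDamageTaken with a zero value rather than the damage dealt, and fires OnDeath whenever health is at zero.
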(event `self.ReceiveBeginPlay`
  (set `self.CurrentHealth` (`self.MaxHealth`)))

(fn `TakeDamage`
  (if (not (`self.bIsInvincible`))
    (set `self.CurrentHealth` (`KismetMathLibrary.FClamp` (- (`self.CurrentHealth`) 20.0) 0.0 (`self.MaxHealth`)))
    (`self.OnDamageTaken` 0.0)
    (if (<= (`self.CurrentHealth`) 0.0)
      (`self.OnDeath`))))