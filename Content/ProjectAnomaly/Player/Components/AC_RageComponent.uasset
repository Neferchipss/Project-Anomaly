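; Player rage component that tracks a rage meter and runs a timed enraged state.
; AddRage adds a fixed, clamped amount only while IsEnraged is already true, and calls ConsumeRage when the meter is full.
; ConsumeRage resets the meter, sets IsEnraged, signals the state's start and starts a duration timer.
; When the timer fires, EndEnragedState clears the flag and signals the end.
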(event `EndEnragedState`
  (set `self.bIsEnraged` false)
  (`self.OnEnragedStateEnd`))

(fn `AddRage`
  (if (`self.bIsEnraged`)
    (set `self.RageCurrent` (`KismetMathLibrary.FClamp` (+ (`self.RageCurrent`) 20.0) 0.0 (`self.RageMax`)))
    (if (>= (`self.RageCurrent`) (`self.RageMax`))
      (`self.ConsumeRage`))))

(fn `ConsumeRage`
  (set `self.bIsEnraged` true)
  (set `self.RageCurrent` 0.0)
  (`self.OnEnragedStateBegin`)
  (bind _returnvalue (`KismetSystemLibrary.K2_SetTimer` null "EndEnragedState" (`self.EnragedDuration`)))
  (set `self.EnragedTimeHandle` _returnvalue))