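; Movement extension component, suffixed OLD, that gives the owning player character a grapple launch.
; TryGrapple line-traces from the player's viewpoint and, if the first hit is a blocking BP_GrappleAnchor, stores it, launches the character and signals attachment.
; The launch vector is owner minus anchor, so it points away from the anchor.
; TryDash is an empty stub, and debug traces and prints remain.
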(fn `TryDash`)

(fn `TryGrapple`
  (bind _returnvalue (`self.GetOwner`))
  (bind _ascharacter (cast `Character` _returnvalue))
  (bind _asplayer_controller (cast `PlayerController` (`Pawn.GetController` _ascharacter)))
  (bind (_location _rotation) (`Controller.GetPlayerViewPoint` _asplayer_controller))
  (bind _outhits (`KismetSystemLibrary.LineTraceMulti` :`Start` _location :`End` (+ _location (* (`self.GrappleRange`) (`KismetMathLibrary.GetForwardVector` _rotation))) :`TraceChannel` "TraceTypeQuery1" :`DrawDebugType` "ForDuration"))
  (bind (_bblockinghit _binitialoverlap _time _distance _location_2 _impactpoint _normal _impactnormal _physmat _hitactor) (`GameplayStatics.BreakHitResult` (`|GetArrayItem` _outhits)))
  (if _bblockinghit
    (`KismetSystemLibrary.PrintString` "e grapple")
    (bind _asbp_grapple_anchor (cast `/Game/ProjectAnomaly/Arena/BP_GrappleAnchor` _hitactor)
      (:`then`
        (bind _output_get (set `self.CurrentAnchor` _asbp_grapple_anchor))
        (`Character.LaunchCharacter` _ascharacter (* (`KismetMathLibrary.Normal` (- (`Actor.K2_GetActorLocation` _returnvalue) (`Actor.K2_GetActorLocation` _output_get))) (`self.GrappleSpeed`)) true true)
        (set `self.bIsGrappling` true)
        (`self.OnGrappleAttached`)
        (return))
      (:`CastFailed`
        (return)))
    (else
      (return))))